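; Spawner actor that periodically spawns Enemy AI pawns at its own location.
; On BeginPlay it starts a looping timer, with the interval rolled once at random between ten and fifteen seconds.
; Each tick of the timer spawns an Enemy with its AI, yawed to face the player pawn.
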(event Custom|SpawnAtLocation
  (AI|SpawnAIFromClass "/Game/Blueprints/Enemy.Enemy_C" 0 (Transformation|GetWorldLocation (Variables|Default|GetDefaultSceneRoot)) (Math|Rotator|MakeRotator 0.0 0.0 (.Yaw (Math|Rotator|BreakRotator (Math|Rotator|FindLookatRotation (Transformation|GetActorLocation) (Transformation|GetActorLocation (Game|Player|GetPlayerPawn 0)))))) false))

(event EventBeginPlay
  (Utilities|Time|SetTimerbyEvent (delegate Custom|SpawnAtLocation) (Math|Random|RandomFloatinRange 1e+01 15.0) true))

(fn ConstructionScript)