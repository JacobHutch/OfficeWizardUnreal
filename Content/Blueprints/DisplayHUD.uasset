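; HUD that draws a crosshair near screen centre plus time dilation and health readouts for the player's FPSController pawn.
; Each DrawHUD call casts the player pawn and reads its Lookin flag to pick the colour of a small square, outlined by four white lines.
; Text labels show the pawn's rounded CustomTimeDilation and its Health, read directly every frame.
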(event EventDrawHUD
  (params (SizeX :type Integer) (SizeY :type Integer))
  (bind _returnvalue (Math|Float|MakeLiteralFloat 8.0))
  (bind _returnvalue_2 (Math|Float|MakeLiteralFloat 1.0))
  (bind _returnvalue_3 (/ SizeY 2))
  (bind _returnvalue_4 (/ SizeX 2))
  (bind _returnvalue_5 (Math|Float|MakeLiteralFloat 4.0))
  (bind _linearcolor (Utilities|Struct|MakeLinearColor 1.0 1.0 1.0 1.0))
  (bind _self self)
  (bind _returnvalue_6 (/ _returnvalue 2.0))
  (bind _returnvalue_7 (Math|Conversions|ToFloat(Integer) _returnvalue_4))
  (bind _returnvalue_8 (Math|Conversions|ToFloat(Integer) _returnvalue_3))
  (bind _returnvalue_9 (- _returnvalue_7 _returnvalue_6))
  (bind _returnvalue_10 (- _returnvalue_8 _returnvalue_6))
  (bind _returnvalue_11 (- _returnvalue_9 _returnvalue_5))
  (bind _returnvalue_12 (- _returnvalue_10 _returnvalue_5))
  (bind _returnvalue_13 (+ _returnvalue_9 _returnvalue_5))
  (bind _returnvalue_14 (+ _returnvalue_10 _returnvalue_5))
  (bind _asfpscontroller (Utilities|Casting|CastToFPSController (Game|Player|GetPlayerPawn 0)))
  (if (Variables|/Game/Blueprints/FPSController.FPSController_C|GetLookin _asfpscontroller)
    (Variables|Default|SetHairColor (Utilities|Struct|MakeLinearColor 1.0 0.0 0.0 1.0))
    (else
      (Variables|Default|SetHairColor (Utilities|Struct|MakeLinearColor 1.0 0.0 0.0 0.0))))
  ;[1 1 1] Crosshair
  (HUD|DrawRect _self (Variables|Default|GetHairColor) (- _returnvalue_7 _returnvalue) (- _returnvalue_8 _returnvalue) _returnvalue _returnvalue)
  (Class|HUD|DrawLine _self _returnvalue_11 _returnvalue_12 _returnvalue_13 _returnvalue_12 _linearcolor _returnvalue_2) ; Top
  (Class|HUD|DrawLine _self _returnvalue_11 _returnvalue_14 _returnvalue_13 _returnvalue_14 _linearcolor _returnvalue_2) ; Bottom
  (Class|HUD|DrawLine _self _returnvalue_11 _returnvalue_12 _returnvalue_11 _returnvalue_14 _linearcolor _returnvalue_2) ; Left
  (Class|HUD|DrawLine _self _returnvalue_13 _returnvalue_12 _returnvalue_13 _returnvalue_14 _linearcolor _returnvalue_2) ; Right
  (HUD|DrawText _self (Utilities|String|Append "DILATION FACTOR: " (Utilities|String|ToString(Integer) (Math|Float|Round (Variables|/Script/Engine.Actor|GetCustomTimeDilation _asfpscontroller))) "x") "(R=1.000000,G=1.000000,B=1.000000,A=1.000000)" 0.0 0.0 "/Game/Montserrat-Regular_Font.Montserrat-Regular_Font" 0.5 false)
  (HUD|DrawText _self (Utilities|String|Append (Utilities|String|MakeLiteralString "HEALTH: ") (Utilities|String|ToString(Integer) (Variables|/Game/Blueprints/FPSController.FPSController_C|GetHealth _asfpscontroller))) "(R=1.000000,G=1.000000,B=1.000000,A=1.000000)" 0.0 35.0 "/Game/Montserrat-Regular_Font.Montserrat-Regular_Font" 0.5 false))

(fn ConstructionScript)