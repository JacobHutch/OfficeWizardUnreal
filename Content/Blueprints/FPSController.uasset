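; First-person player character with look, sprint, double jump, physics object grab/throw and adjustable slow motion, which adds the MenuHUD widget on BeginPlay.
; Tick traces from the camera to set the Lookin flag and teleports held objects to the Hold point.
; Dropping cancels the object's velocity, then launches it forward with time-dilation-scaled force.
; Slow motion lowers global time dilation while inverse CustomTimeDilation keeps the player at normal speed.
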(event Custom|PickupObject
  (bind _camera (Variables|Default|GetCamera))
  (bind _returnvalue (Transformation|GetWorldLocation _camera))
  ;[1 1 1] Grab/Drop
  (bind (_outhit _returnvalue_2) (Collision|LineTraceForObjects _returnvalue (+ (* (Math|Vector|GetForwardVector _camera) 3e+02) _returnvalue) (Utilities|Array|MakeArray "ObjectTypeQuery4") false 0 "None" true "(R=0.000000,G=0.000000,B=0.000000,A=0.000000)" "(R=0.000000,G=0.000000,B=0.000000,A=0.000000)" 0.0))
  (if _returnvalue_2
    (if (Physics|IsSimulatingPhysics (.HitComponent (Collision|BreakHitResult _outhit)) "None")
      (Class|PhysicsHandleComponent|GrabComponentatLocation (Variables|Default|GetPhysicsHandle) (.HitComponent (Collision|BreakHitResult _outhit)) "None" (Transformation|GetWorldLocation (.HitComponent (Collision|BreakHitResult _outhit))))
      (Variables|Default|SetIsHoldingObject true)
      (Variables|Default|SetLookin true))))

(event Custom|DropObject
  ;[1 1 1] Grab/Drop
  (Physics|Components|PhysicsHandle|ReleaseComponent (Variables|Default|GetPhysicsHandle))
  (Physics|AddImpulse (.HitComponent (Collision|BreakHitResult (stale Custom|PickupObject _outhit))) (- "0, 0, 0" (Transformation|GetComponentVelocity (.HitComponent (Collision|BreakHitResult (stale Custom|PickupObject _outhit))))) "None" true)
  (Physics|AddImpulse (.HitComponent (Collision|BreakHitResult (stale Custom|PickupObject _outhit))) (* (Math|Vector|GetForwardVector (Variables|Default|GetCamera)) (/ 1e+03 (Math|Float|Power (Class|GameplayStatics|GetGlobalTimeDilation) 0.2))) "None" true)
  (Variables|Default|SetIsHoldingObject false))

(event Custom|Trace
  (bind _camera (Variables|Default|GetCamera))
  (bind _isholdingobject (Variables|Default|GetIsHoldingObject))
  (bind _returnvalue (Transformation|GetWorldLocation _camera))
  (bind _returnvalue_2 (or _isholdingobject false))
  ;[1 1 1] Grab/Drop
  (bind (_outhit _returnvalue_3) (Collision|LineTraceForObjects _returnvalue (+ (* (Math|Vector|GetForwardVector _camera) 3e+02) _returnvalue) (Utilities|Array|MakeArray "ObjectTypeQuery4") false 0 "None" true "(R=0.000000,G=0.000000,B=0.000000,A=0.000000)" "(R=0.000000,G=0.000000,B=0.000000,A=0.000000)" 0.0))
  (if _returnvalue_3
    (if (Physics|IsSimulatingPhysics (.HitComponent (Collision|BreakHitResult _outhit)) "None")
      (Variables|Default|SetLookin true)
      (else
        (Variables|Default|SetLookin _returnvalue_2)))
    (else
      (Variables|Default|SetLookin _returnvalue_2))))

(event Custom|Teleport
  ;[1 1 1] Grab/Drop
  (if (Variables|Default|GetIsHoldingObject)
    (Transformation|Teleport (.HitActor (Collision|BreakHitResult (stale Custom|PickupObject _outhit))) (Transformation|GetWorldLocation (Variables|Default|GetHold)) "0, 0, 0")))

(event Custom|DeathTime)

(event EventOnLanded
  (params (Hit :type Hit%20Result%20Structure%20%28by%20ref%29))
  ;[1 1 1] Jump/DoubleJump
  (Utilities|FlowControl|DoN 2) ; enters at Reset
)

(event EventBeginPlay
  (bind _returnvalue (UserInterface|CreateWidget "/Game/Blueprints/MenuHUD.MenuHUD_C"))
  (bind _output_get (Variables|Default|SetMainHUDReference _returnvalue))
  (UserInterface|Viewport|AddtoViewport _output_get 0)
  (Input|SetInputModeGameOnly (Game|GetPlayerController 0)))

(event EventTick
  (params (DeltaSeconds :type Float%20%28single-precision%29))
  ;[1 1 1] Event Tick Functions
  (CallFunction|Trace)
  (CallFunction|Teleport))

(event Input|ActionEvents|InputActionJump
  (params (Key :type Key%20Structure))
  ;[1 1 1] Jump/DoubleJump
  (:Pressed
    (bind _counter (Utilities|FlowControl|DoN 2)
      (:Exit
        (switch int _counter
          (:1
            (Character|Jump))
          (:2
            (Character|LaunchCharacter "0, 0,600.000000" false false)))))))

(event Input|ActionEvents|InputActionTimeSpeed
  (params (Key :type Key%20Structure))
  ;[1 1 1] Time Dilation
  (:Pressed
    (bind _output_get (Variables|Default|SetTimeDilation (Math|Float|Clamp(Float) (* (Variables|Default|GetTimeDilation) (Variables|Default|GetFactor)) 0.0001 0.1)))
    (if (Variables|Default|GetActivate)
      (Utilities|Time|SetGlobalTimeDilation _output_get)
      (Variables|Default|SetCustomTimeDilation (/ 1.0 _output_get)))))

(event Input|ActionEvents|InputActionTimeSlow
  (params (Key :type Key%20Structure))
  ;[1 1 1] Time Dilation
  (:Pressed
    (bind _output_get (Variables|Default|SetTimeDilation (Math|Float|Clamp(Float) (/ (Variables|Default|GetTimeDilation) (Variables|Default|GetFactor)) 0.0001 0.1)))
    (if (Variables|Default|GetActivate)
      (Utilities|Time|SetGlobalTimeDilation _output_get)
      (Utilities|FlowControl|Delay 1e-05)
      (Variables|Default|SetCustomTimeDilation (/ 1.0 _output_get)))))

(event Input|ActionEvents|InputActionTimeActivate
  (params (Key :type Key%20Structure))
  (bind _timedilation (Variables|Default|GetTimeDilation))
  ;[1 1 1] Time Dilation
  (:Pressed
    (Utilities|FlowControl|FlipFlop
      (:A
        (Variables|Default|SetActivate true)
        (Utilities|Time|SetGlobalTimeDilation _timedilation)
        (Utilities|FlowControl|Delay 1e-05)
        (Variables|Default|SetCustomTimeDilation (/ 1.0 _timedilation)))
      (:B
        (Variables|Default|SetActivate false)
        (Utilities|Time|SetGlobalTimeDilation 1.0)
        (Variables|Default|SetCustomTimeDilation 1.0)))))

(event Input|ActionEvents|InputActionSprint
  (params (Key :type Key%20Structure))
  (bind _charactermovement (Variables|Character|GetCharacterMovement))
  ;[1 1 1] Movement
  (:Pressed
    (Variables|/Script/Engine.CharacterMovementComponent|SetMaxWalkSpeed _charactermovement 1.2e+03))
  (:Released
    (Variables|/Script/Engine.CharacterMovementComponent|SetMaxWalkSpeed _charactermovement 6e+02)))

(event Input|AxisEvents|InputAxisLookHorizontal
  (params (AxisValue :type Float%20%28single-precision%29))
  ;[1 1 1] Look
  (Pawn|Input|AddControllerYawInput AxisValue))

(event Input|AxisEvents|InputAxisLookVertical
  (params (AxisValue :type Float%20%28single-precision%29))
  ;[1 1 1] Look
  (Pawn|Input|AddControllerPitchInput AxisValue))

(event Input|AxisEvents|InputAxisMoveVertical
  (params (AxisValue :type Float%20%28single-precision%29))
  ;[1 1 1] Movement
  (Pawn|Input|AddMovementInput (Math|Vector|GetForwardVector (Math|Rotator|MakeRotator 0.0 0.0 (.yaw (Pawn|GetControlRotation :!class /Script/Engine.Pawn)))) AxisValue false))

(event Input|AxisEvents|InputAxisMoveHorizontal
  (params (AxisValue :type Float%20%28single-precision%29))
  ;[1 1 1] Movement
  (Pawn|Input|AddMovementInput (Math|Vector|GetRightVector (Math|Rotator|MakeRotator 0.0 0.0 (.yaw (Pawn|GetControlRotation :!class /Script/Engine.Pawn)))) AxisValue false))

(event Input|MouseEvents|LeftMouseButton
  (params (Key :type Key%20Structure))
  ;[1 1 1] Grab/Drop
  (:Pressed
    (if (Variables|Default|GetIsHoldingObject)
      (CallFunction|DropObject)
      (else
        (CallFunction|PickupObject)))))

(fn ConstructionScript)