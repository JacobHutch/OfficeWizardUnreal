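; Enemy character that chases the player on sight and can be killed by physics impacts.
; Pawn sensing starts an AI move to the FPSController; reaching it removes one Health unless Activate or Dead is set, triggering DeathTime at zero.
; Hits involving a physics-simulating component launch the enemy along the impact normal with upward lift, remove one Health and destroy it at zero.
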(event OnSeePawn(PawnSensing)
  (params (Pawn :type Pawn%20Object%20Reference))
  (bind _asfpscontroller (Utilities|Casting|CastToFPSController Pawn))
  (AI|AIMoveTo self "0, 0, 0" _asfpscontroller 5.0 true
    (:OnSuccess
      (if (not (Variables|/Game/Blueprints/FPSController.FPSController_C|GetActivate _asfpscontroller))
        (if (not (Variables|/Game/Blueprints/FPSController.FPSController_C|GetDead _asfpscontroller))
          (bind _output_get (Variables|/Game/Blueprints/FPSController.FPSController_C|SetHealth _asfpscontroller (- (Variables|/Game/Blueprints/FPSController.FPSController_C|GetHealth _asfpscontroller) 1)))
          (if (not (> _output_get 0))
            (Variables|/Game/Blueprints/FPSController.FPSController_C|SetDead _asfpscontroller true)
            (Default|DeathTime _asfpscontroller)))))))

(event Collision|EventHit
  (params (MyComp :type Primitive%20Component%20Object%20Reference) (Other :type Actor%20Object%20Reference) (OtherComp :type Primitive%20Component%20Object%20Reference) (bSelfMoved :type Boolean) (HitLocation :type Vector :default "0, 0, 0") (HitNormal :type Vector :default "0, 0, 0") (NormalImpulse :type Vector :default "0, 0, 0") (Hit :type Hit%20Result%20Structure%20%28by%20ref%29))
  (bind (_bblockinghit _binitialoverlap _time _distance _location _impactpoint _normal _impactnormal _physmat _hitactor _hitcomponent) (Collision|BreakHitResult Hit))
  (bind _returnvalue (* _impactnormal 5e+02))
  (bind (_x _y) (Math|Vector|BreakVector _returnvalue))
  (if (Physics|IsSimulatingPhysics _hitcomponent "None")
    (Character|LaunchCharacter (Math|Vector|MakeVector _x _y 2e+02) false true)
    (bind _output_get (Variables|Default|SetHealth (- (Variables|Default|GetHealth) 1)))
    (if (== _output_get 0)
      (Actor|DestroyActor))))

(fn ConstructionScript)